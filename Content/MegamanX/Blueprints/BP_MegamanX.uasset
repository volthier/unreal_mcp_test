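; BP_MegamanX is a player-controlled Mega Man X character with mouse look, WASD movement and jumping.
; All logic runs on Tick, polling player controller 0 directly for mouse delta and key states with hardcoded keys.
; Mouse delta drives controller yaw and inverted-sign pitch, while movement follows the yaw-only control rotation and Space calls Jump.
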(event EventBeginPlay)

(event Collision|EventActorBeginOverlap
  (params (OtherActor :type Actor%20Object%20Reference)))

(event EventTick
  (params (DeltaSeconds :type Float%20%28single-precision%29))
  (bind _returnvalue (Game|GetPlayerController 0))
  (bind _self self)
  (bind (_deltax _deltay) (Class|PlayerController|GetInputMouseDelta _returnvalue))
  (bind _returnvalue_2 (Pawn|GetControlRotation _returnvalue :!class /Script/Engine.Controller))
  (bind _yaw (Math|Rotator|BreakRotator _returnvalue_2))
  (bind _returnvalue_3 (Math|Rotator|MakeRotator 0.0 0.0 _yaw))
  (bind _returnvalue_4 (Math|Vector|GetForwardVector _returnvalue_3))
  (bind _returnvalue_5 (Math|Vector|GetRightVector _returnvalue_3))
  (Pawn|Input|AddControllerYawInput _self _deltax)
  (Pawn|Input|AddControllerPitchInput _self (- 0.0 _deltay))
  (if (Game|Player|IsInputKeyDown _returnvalue "W")
    (Pawn|Input|AddMovementInput _self _returnvalue_4 1.0 false))
  (if (Game|Player|IsInputKeyDown _returnvalue "S")
    (Pawn|Input|AddMovementInput _self _returnvalue_4 -1.0 false))
  (if (Game|Player|IsInputKeyDown _returnvalue "D")
    (Pawn|Input|AddMovementInput _self _returnvalue_5 1.0 false))
  (if (Game|Player|IsInputKeyDown _returnvalue "A")
    (Pawn|Input|AddMovementInput _self _returnvalue_5 -1.0 false))
  (if (Game|Player|IsInputKeyDown _returnvalue "SpaceBar")
    (Character|Jump _self)))

(fn ConstructionScript)