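; BP_ClericPlayer is the Cleric player character, with left/right movement along world X and jumping.
; BeginPlay prints a debug label, sets the mesh to Animation Blueprint mode, adds the IMC_VoltStriker Enhanced Input context to player 0 and applies one +X movement input.
; Tick polls action values rather than binding input events, feeding right minus left into movement input and calling Jump while the jump action is active.
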(event EventBeginPlay
  (Development|PrintString "Cleric")
  (Components|Animation|SetAnimationMode (Variables|Character|GetMesh) "AnimationBlueprint" true)
  (Input|AddMappingContext (PlayerController|LocalPlayerSubsystems|GetEnhancedInputLocalPlayerSubsystem (Game|GetPlayerController 0)) "/Game/VoltStriker/Input/IMC_VoltStriker.IMC_VoltStriker" 0 "(bIgnoreAllPressedKeysUntilRelease=True,bForceImmediately=False,bNotifyUserSettings=False)")
  (Pawn|Input|AddMovementInput "1.000000,0.000000,0.000000" 1.0 false))

(event Collision|EventActorBeginOverlap
  (params (OtherActor :type Actor%20Object%20Reference)))

(event EventTick
  (params (DeltaSeconds :type Float%20%28single-precision%29))
  (Pawn|Input|AddMovementInput "1.000000,0.000000,0.000000" (- (Input|EnhancedActionValues|GetIA_MoveRight) (Input|EnhancedActionValues|GetIA_MoveLeft)) false)
  (if (Input|EnhancedActionValues|GetIA_Jump)
    (Character|Jump)))

(fn ConstructionScript)