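; BP_PlayerRobot is the player-controlled robot character in VoltStriker, handling basic movement and jumping.
; BeginPlay switches the mesh to custom animation mode and adds the IMC_VoltStriker Enhanced Input mapping context for player 0.
; Tick polls input action values, combining opposing actions into forward and right axes relative to control yaw, and calls Jump while the jump action is active.
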(event EventBeginPlay
  (Development|PrintString "VoltStriker ready" true true "(R=0.000000,G=0.660000,B=1.000000,A=1.000000)" 5.0)
  (Components|Animation|SetAnimationMode (Variables|Character|GetMesh) "AnimationCustomMode" false)
  (Input|AddMappingContext (PlayerController|LocalPlayerSubsystems|GetEnhancedInputLocalPlayerSubsystem (Game|GetPlayerController 0)) "/Game/VoltStriker/Input/IMC_VoltStriker.IMC_VoltStriker" 0 "(bIgnoreAllPressedKeysUntilRelease=True,bForceImmediately=False,bNotifyUserSettings=False)"))

(event Collision|EventActorBeginOverlap
  (params (OtherActor :type Actor%20Object%20Reference)))

(event EventTick
  (params (DeltaSeconds :type Float%20%28single-precision%29))
  (bind _returnvalue (Pawn|GetController))
  (bind _returnvalue_2 (Pawn|GetControlRotation _returnvalue :!class /Script/Engine.Controller))
  (bind _yaw (Math|Rotator|BreakRotator _returnvalue_2))
  (bind _returnvalue_3 (Math|Rotator|MakeRotator 0.0 0.0 _yaw))
  (Pawn|Input|AddMovementInput (Math|Vector|GetForwardVector _returnvalue_3) (- (Input|EnhancedActionValues|GetIA_MoveForward) (Input|EnhancedActionValues|GetIA_MoveBack)) false)
  (Pawn|Input|AddMovementInput (Math|Vector|GetRightVector _returnvalue_3) (- (Input|EnhancedActionValues|GetIA_MoveRight) (Input|EnhancedActionValues|GetIA_MoveLeft)) false)
  (if (Input|EnhancedActionValues|GetIA_Jump)
    (Character|Jump)))

(fn ConstructionScript)